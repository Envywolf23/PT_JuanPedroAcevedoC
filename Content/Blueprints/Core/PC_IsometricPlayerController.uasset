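; Player controller for the isometric building minigame, handling mouse selection and drag placement of buildings.
; It adds the Enhanced Input mapping context, shows the cursor and caches the minigame game state.
; Clicks trace under the cursor to start dragging the ghost actor or select a building through the placeable interface.
; While the game state is Dragging, Tick moves the ghost to the cursor hit; releasing switches it to WaitingConfirm.
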(event `self.ReceiveBeginPlay`
  (bind _returnvalue (subsystem `EnhancedInputLocalPlayerSubsystem`))
  ; Begin Play
  (`/Engine/EditorBlueprintResources/StandardMacros.IsValid` _returnvalue
    (:`Is Valid`
      (`EnhancedInputSubsystemInterface.AddMappingContext` _returnvalue "/Game/Blueprints/Input/IMC_IsometricMinigame.IMC_IsometricMinigame" 0 (struct))
      (set `self.bShowMouseCursor` true)
      (bind _asgs_isometric_minigame (cast `/Game/Blueprints/Core/GS_IsometricMinigame` (`GameplayStatics.GetGameState`)))
      (set `self.GS Isometric Reference` _asgs_isometric_minigame))))

(event `EnhancedInput|/Game/Blueprints/Input/Actions/IA_Select_Click`
  (params (ActionValue :type Boolean) (ElapsedSeconds :type "Float (double-precision)") (TriggeredSeconds :type "Float (double-precision)") (InputAction :type "InputAction Object Reference" :default "/Game/Blueprints/Input/Actions/IA_Select_Click.IA_Select_Click"))
  (bind (_hit _location _actor) (`self.GetActorUnderCursor`))
  (bind _gs_isometric_reference (`self.GS Isometric Reference`))
  ;[0.4115 0.1717 0.00082 0.5] INPUT: Selection_Click
  (:`Started`
    (set `self.ActorUnderCursor` _actor)
    (if _hit
      (if (== (`/Game/Blueprints/Core/GS_IsometricMinigame.GhostActor` (`self.GS Isometric Reference`)) (`self.ActorUnderCursor`))
        (`self.HandleGhostClick`)
        (else
          (`self.Handle Building Click`)))))
  (:`Completed`
    (`self.onPlayerStopDrag`)
    (if (`|EnumEquality` (`/Game/Blueprints/Core/GS_IsometricMinigame.CurrentState` _gs_isometric_reference) "NewEnumerator1")
      (set `/Game/Blueprints/Core/GS_IsometricMinigame.CurrentState` "NewEnumerator2" _gs_isometric_reference))))

(event `HandleGhostClick`
  (bind _gs_isometric_reference (`self.GS Isometric Reference`))
  ;[0.4115 0.1717 0.00082 0.5] Handle Ghost Click
  (if (`KismetSystemLibrary.DoesImplementInterface` (`self.ActorUnderCursor`) "/Game/Blueprints/Buildings/BPI_Placeable.BPI_Placeable_C")
    (set `/Game/Blueprints/Core/GS_IsometricMinigame.CurrentState` "NewEnumerator1" _gs_isometric_reference)
    (`/Game/Blueprints/Buildings/BPI_Placeable.onStartDrag` (`/Game/Blueprints/Core/GS_IsometricMinigame.GhostActor` _gs_isometric_reference))))

(event `Handle Building Click`
  (bind _actorundercursor (`self.ActorUnderCursor`))
  ;[0.4115 0.1717 0.00082 0.5] Handle Building Click
  (bind _asbp_building_base (cast `/Game/Blueprints/Buildings/BP_BuildingBase` _actorundercursor))
  (if (`KismetSystemLibrary.DoesImplementInterface` _actorundercursor "/Game/Blueprints/Buildings/BPI_Placeable.BPI_Placeable_C")
    (`/Game/Blueprints/Buildings/BPI_Placeable.onSelected` _asbp_building_base)))

(event `self.ReceiveTick`
  (params (DeltaSeconds :type "Float (single-precision)"))
  (bind (_hit _location) (`self.GetActorUnderCursor`))
  ;[0.15 0.1345 0] Event Tick
  (switch `/Game/Blueprints/Core/EPlacementState` (`/Game/Blueprints/Core/GS_IsometricMinigame.CurrentState` (`self.GS Isometric Reference`))
    (:`NewEnumerator1`
      (if _hit
        (`self.K2_SetActorLocation` (`/Game/Blueprints/Core/GS_IsometricMinigame.GhostActor` (`self.GS Isometric Reference`)) (`KismetMathLibrary.MakeVector` (.x _location) (.y _location)) false false)))))

(fn `GetActorUnderCursor`
  (returns (Hit :type Boolean) (Location :type "Vector Structure") (Actor :type "Actor Object Reference"))
  (bind (_bblockinghit _binitialoverlap _time _distance _location _impactpoint _normal _impactnormal _physmat _hitactor) (`GameplayStatics.BreakHitResult` (`self.GetHitResultUnderCursorByChannel` "TraceTypeQuery1")))
  (return _bblockinghit _location _hitactor))

(fn `UserConstructionScript`)