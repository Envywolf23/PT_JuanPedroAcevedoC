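; Game State for the isometric minigame that runs building placement.
; BeginPlacement, when idle, spawns the chosen building as a ghost actor, starts its drag, binds its positioning-finished event and switches to a placing state.
; ClearGhostActor unbinds and releases the ghost, returns to idle and saves all buildings through GI_SaveManager.
; A helper returns the Visibility-channel hit under the cursor; Delete is an empty stub.
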(event `BeginPlacement`
  (params (BuildingType :type "/Game/Blueprints/Buildings/BP_BuildingBase Class Reference"))
  ;[0.15 0.007745 0 0.5] BeginPlacement Logic
  (if (`|EnumEquality` (`self.CurrentState`) "NewEnumerator0")
    (bind _returnvalue (`|SpawnActorFromClass` BuildingType (`KismetMathLibrary.MakeTransform` (0.0 0.0 0.0)) "Undefined" "MultiplyWithRoot" null null))
    (bind _output_get (set `self.GhostActor` _returnvalue))
    (`/Game/Blueprints/Buildings/BPI_Placeable.onStartDrag` _output_get)
    (add `/Game/Blueprints/Buildings/BP_BuildingBase.onPositioningFinished` _output_get (`|CreateDelegate` :!event `ClearGhostActor`))
    (set `self.CurrentState` "NewEnumerator1")))

(event `ClearGhostActor`
  ; Clear Ghost Actor
  (remove `/Game/Blueprints/Buildings/BP_BuildingBase.onPositioningFinished` (`self.GhostActor`) (`|CreateDelegate` :!event `ClearGhostActor`))
  (set `self.GhostActor` null)
  (set `self.CurrentState` "NewEnumerator0")
  (bind _asgi_save_manager (cast `/Game/Blueprints/Core/GameData/GI_SaveManager` (`GameplayStatics.GetGameInstance`)))
  (`/Game/Blueprints/Core/GameData/GI_SaveManager.SaveAllBuildings` _asgi_save_manager))

(event `Delete`)

(fn `GetActorUnderCursor`
  (returns (Hit :type Boolean) (Location :type "Vector Structure") (Actor :type "Actor Object Reference"))
  (bind _aspc_isometric_player_controller (cast `/Game/Blueprints/Core/PC_IsometricPlayerController` (`GameplayStatics.GetPlayerController` 0)))
  (bind (_bblockinghit _binitialoverlap _time _distance _location _impactpoint _normal _impactnormal _physmat _hitactor) (`GameplayStatics.BreakHitResult` (`PlayerController.GetHitResultUnderCursorByChannel` _aspc_isometric_player_controller "TraceTypeQuery1" false)))
  (return _bblockinghit _location _hitactor))

(fn `UserConstructionScript`)